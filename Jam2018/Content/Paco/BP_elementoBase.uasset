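; BP_elementoBase is a base element actor with a static mesh that gets a random color and is pushed when play begins.
; The construction script creates a dynamic material instance from the mesh's first material and sets its Color parameter, randomizing each RGB channel between configurable min and max range variables.
; BeginPlay applies a fixed, mass-dependent impulse to the mesh, mostly along world X.
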(event EventBeginPlay
  (Physics|AddImpulse (Variables|Default|GetStaticMesh) "500.000000,10.000000,10.000000" "None" false))

(event Collision|EventActorBeginOverlap
  (params (OtherActor :type Actor%20Object%20Reference)))

(event EventTick
  (params (DeltaSeconds :type Float%20%28single-precision%29)))

(fn ConstructionScript
  (bind _minrangecolor (Variables|Default|GetMinRangeColor))
  (bind _maxrangecolor (Variables|Default|GetMaxRangeColor))
  (Utilities|FlowControl|Sequence
    (:then_0
      ;[1 1 1] Color Random Por Rangos
      (bind _returnvalue (Rendering|Material|CreateDynamicMaterialInstance (Variables|Default|GetStaticMesh) 0 (Rendering|Material|GetMaterial (Variables|Default|GetStaticMesh) 0) :!class /Script/Engine.PrimitiveComponent))
      (Variables|Default|SetM_ElementoBase_Inst _returnvalue)
      (Rendering|Material|SetVectorParameterValue _returnvalue "Color" (Math|Conversions|ToLinearColor(Vector) (Math|Vector|MakeVector (Math|Random|RandomFloatinRange _minrangecolor _maxrangecolor) (Math|Random|RandomFloatinRange _minrangecolor _maxrangecolor) (Math|Random|RandomFloatinRange _minrangecolor _maxrangecolor))) :!class /Script/Engine.MaterialInstanceDynamic)
      (Rendering|Material|SetMaterial (Variables|Default|GetStaticMesh) 0 _returnvalue))))