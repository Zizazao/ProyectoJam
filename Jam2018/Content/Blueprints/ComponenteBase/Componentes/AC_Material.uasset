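; Component that randomizes the look of a component's static mesh and particle system when MaterialUpdate is called, handling only the Subatomico type.
; It creates a dynamic material instance and loops ArrayProperties, using enum names as parameter names for random colors or ranged scalars.
; It also gives the particle system's point and trail materials random colors.
; Color channels are random 0–255 values passed straight to linear color, without normalization.
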(event Custom|MaterialUpdate
  (params (StaticMesh :type Static%20Mesh%20Component%20Object%20Reference) (ParticleSystem :type Particle%20System%20Component%20Object%20Reference) (ComponentType :type E_TiposComponente%20Enum :default "NewEnumerator5"))
  (bind _returnvalue (Rendering|Material|GetMaterial StaticMesh 0))
  (Variables|Default|SetTipoComp ComponentType)
  (Variables|Default|SetParticleSystem ParticleSystem)
  (bind _output_get (Variables|Default|SetStaticMesh StaticMesh))
  (Variables|Default|SetMaterial _returnvalue)
  (bind _returnvalue_2 (Rendering|Material|CreateDynamicMaterialInstance _output_get 0 _returnvalue :!class /Script/Engine.PrimitiveComponent))
  (Variables|Default|SetDynamicInstance _returnvalue_2)
  ;[1 1 1] Para cada material hacer logica correspondiente
  (switch Utilities|FlowControl|Switch|SwitchonE_TiposComponente (Variables|Default|GetTipoComp)
    (:NewEnumerator0
      (for _array_element (Variables|Default|GetArrayProperties)
        ;[1 1 1] Setear las Variables del Material Dinamicamente
        (if (.HasColor (Utilities|Struct|BreakS_SubAtomicoProperties _array_element))
          (Rendering|Material|SetVectorParameterValue (Variables|Default|GetDynamicInstance) (Utilities|String|StringToName (Utilities|String|EnumtoString (.Property (Utilities|Struct|BreakS_SubAtomicoProperties _array_element)))) (Math|Conversions|ToLinearColor(Vector) (Math|Vector|MakeVector (Math|Random|RandomFloatinRange 0.0 255.0) (Math|Random|RandomFloatinRange 0.0 255.0) (Math|Random|RandomFloatinRange 0.0 255.0))) :!class /Script/Engine.MaterialInstanceDynamic)
          (else
            (Rendering|Material|SetScalarParameterValue (Variables|Default|GetDynamicInstance) (Utilities|String|StringToName (Utilities|String|EnumtoString (.Property (Utilities|Struct|BreakS_SubAtomicoProperties _array_element)))) (Math|Random|RandomFloatinRange (.Min (Utilities|Struct|BreakS_SubAtomicoProperties _array_element)) (.Max (Utilities|Struct|BreakS_SubAtomicoProperties _array_element))) :!class /Script/Engine.MaterialInstanceDynamic))))
      (Rendering|Material|SetMaterial (Variables|Default|GetStaticMesh) 0 (Variables|Default|GetDynamicInstance))
      (Utilities|FlowControl|Sequence
        (:then_1
          ;[1 1 1] Color random de punto de particulas por rango
          (bind _returnvalue_3 (Rendering|Material|CreateDynamicMaterialInstance (Variables|Default|GetParticleSystem) 0 (Rendering|Material|GetMaterial (Variables|Default|GetParticleSystem) 0) :!class /Script/Engine.PrimitiveComponent))
          (Rendering|Material|SetVectorParameterValue _returnvalue_3 "ParticleColorParam" (Math|Conversions|ToLinearColor(Vector) (Math|Vector|MakeVector (Math|Random|RandomFloatinRange 0.0 255.0) (Math|Random|RandomFloatinRange 0.0 255.0) (Math|Random|RandomFloatinRange 0.0 255.0))) :!class /Script/Engine.MaterialInstanceDynamic)
          (Rendering|Material|SetMaterial (Variables|Default|GetParticleSystem) 0 _returnvalue_3))
        (:then_2
          ;[1 1 1] Color Particulas Trail
          (bind _returnvalue_4 (Rendering|Material|CreateDynamicMaterialInstance (Variables|Default|GetParticleSystem) 1 (Rendering|Material|GetMaterial (Variables|Default|GetParticleSystem) 1) :!class /Script/Engine.PrimitiveComponent))
          (Rendering|Material|SetVectorParameterValue _returnvalue_4 "TrailColor" (Math|Conversions|ToLinearColor(Vector) (Math|Vector|MakeVector (Math|Random|RandomFloatinRange 0.0 255.0) (Math|Random|RandomFloatinRange 0.0 255.0) (Math|Random|RandomFloatinRange 0.0 255.0))) :!class /Script/Engine.MaterialInstanceDynamic)
          (Rendering|Material|SetMaterial (Variables|Default|GetParticleSystem) 1 _returnvalue_4))))))