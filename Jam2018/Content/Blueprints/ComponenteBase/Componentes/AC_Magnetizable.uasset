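; Actor component that makes its owner magnetizable, pulling its mesh toward a given hand location.
; The Atraer (attract) event finds the owner's StaticMeshComponent and uses MoveComponentTo to glide it over a fixed duration with ease-in and ease-out.
; The hand location is passed directly as the target relative location.
; Distance-scaling and transform-easing nodes are present but unused.
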(event Custom|Atraer
  (params (LocalizacionMano :type Vector))
  (Components|MoveComponentTo (Actor|GetComponentbyClass (Components|GetOwner) "/Script/Engine.StaticMeshComponent") LocalizacionMano "0, 0, 0" true true 3.0 false))