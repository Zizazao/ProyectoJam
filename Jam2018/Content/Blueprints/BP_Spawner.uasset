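; BP_Spawner is an actor that scatters spawned actors at random positions, filling the scene with a batch of BP_Subatomicos on BeginPlay.
; A FillScene event spawns one actor of a given class through the same Generator function.
; The construction script sizes the Sphere from SpawnerSize; Generator uses that radius as per-axis random bounds, giving a cubic volume around world origin, since no actor location is added.
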(event Custom|FillScene
  (params (ActorToFill :type Actor%20Class%20Reference))
  (CallFunction|Generator ActorToFill))

(event EventBeginPlay
  (for _index (range 0 150)
    (CallFunction|Generator "/Game/Blueprints/01_Subatomicos/BP_Subatomicos.BP_Subatomicos_C")))

(event Collision|EventActorBeginOverlap
  (params (OtherActor :type Actor%20Object%20Reference)))

(event EventTick
  (params (DeltaSeconds :type Float%20%28single-precision%29)))

(fn ConstructionScript
  (Components|Sphere|SetSphereRadius (Variables|Default|GetSphere) (Variables|Default|GetSpawnerSize) true))

(fn Generator
  (params (ActorClass :type Actor%20Class%20Reference))
  (bind _sphere (Variables|Default|GetSphere))
  (bind _sphereradius (Variables|/Script/Engine.SphereComponent|GetSphereRadius _sphere))
  (bind _returnvalue (* _sphereradius -1.0))
  (bind _returnvalue_2 (Game|SpawnActorfromClass ActorClass (Math|Transform|MakeTransform (Math|Vector|MakeVector (Math|Random|RandomFloatinRange _returnvalue _sphereradius) (Math|Random|RandomFloatinRange _returnvalue _sphereradius) (Math|Random|RandomFloatinRange _returnvalue _sphereradius)) "0, 0, 0" "1,1,1") "Undefined" self 0))
  (AddComponent|AddChildActorComponent _returnvalue_2 false))