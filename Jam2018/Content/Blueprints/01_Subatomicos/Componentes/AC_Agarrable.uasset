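; AC_Agarrable is an actor component that lets its owner, apparently a subatomic object, be picked up and dropped.
; PickUp disables the mesh's physics, deactivates the owner's AC_MovimientoSub and snaps the mesh to the middle_01_r socket, hard-coded to a right-hand finger, on the given component.
; Drop restores physics, detaches the mesh keeping its world transform and reactivates that movement component.
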(event Custom|PickUp
  (params (MeshToPickUp :type Static%20Mesh%20Component%20Object%20Reference) (AttachTo :type Skeletal%20Mesh%20Component%20Object%20Reference))
  (Physics|SetSimulatePhysics MeshToPickUp false)
  (Components|Activation|Deactivate (Actor|GetComponentbyClass (Components|GetOwner) "/Game/Blueprints/01_Subatomicos/Componentes/AC_MovimientoSub.AC_MovimientoSub_C"))
  (Transformation|AttachComponentToComponent MeshToPickUp AttachTo "middle_01_r" "SnapToTarget" "SnapToTarget" "SnapToTarget" false))

(event Custom|Drop
  (params (Mesh%20ToDetach :type Static%20Mesh%20Component%20Object%20Reference))
  (Physics|SetSimulatePhysics Mesh%20ToDetach true)
  (Transformation|DetachFromComponent Mesh%20ToDetach "KeepWorld" "KeepWorld" "KeepWorld" true)
  (Components|Activation|Activate (Actor|GetComponentbyClass (Components|GetOwner) "/Game/Blueprints/01_Subatomicos/Componentes/AC_MovimientoSub.AC_MovimientoSub_C") false))