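; BP_Subatomico is a grabbable subatomic particle actor that drifts around the scene.
; On BeginPlay it sets a fixed grab pose and animation, activates its particle system after a short delay, and applies a random impulse through ACMovimiento.
; A looping timer repeats that impulse at an interval randomized once per instance.
; When its mesh stops overlapping a BP_Spawner, it passes its class to FillScene on that spawner and destroys itself.
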(event OnComponentEndOverlap(StaticMesh)
  (params (OverlappedComponent :type Primitive%20Component%20Object%20Reference) (OtherActor :type Actor%20Object%20Reference) (OtherComp :type Primitive%20Component%20Object%20Reference) (OtherBodyIndex :type Integer))
  (bind _asbp_spawner (Utilities|Casting|CastToBP_Spawner OtherActor))
  (Default|FillScene _asbp_spawner (Utilities|GetClass self))
  (Actor|DestroyActor))

(event EventBeginPlay
  (bind _returnvalue (Math|Transform|MakeTransform "2.100000,0.200000,9.700000" "73.000000,111.000000,178.000000"))
  (|CallParentFunction)
  (Utilities|FlowControl|Sequence
    (:then_0
      (Utilities|FlowControl|Delay 0.2)
      (Components|Activation|Activate (Variables|Default|GetParticleSystem) false))
    (:then_1
      (Default|SetFixedGrab (Variables|Default|GetGrabable) (Variables|Default|GetStaticMesh) _returnvalue "/Game/Framework/Hands/Model/Animations/Grabs/grab_round_medium.grab_round_medium" _returnvalue)
      (Default|AddImpulseRandom (Variables|Default|GetAC_Movimiento))
      (Utilities|Time|SetTimerbyFunctionName (Variables|Default|GetAC_Movimiento) "AddImpulseRandom" (Math|Random|RandomFloatinRange 0.0 8.0) true))))

(event Collision|EventActorBeginOverlap
  (params (OtherActor :type Actor%20Object%20Reference)))

(event EventTick
  (params (DeltaSeconds :type Float%20%28single-precision%29)))

(fn ConstructionScript
  (|CallParentFunction))