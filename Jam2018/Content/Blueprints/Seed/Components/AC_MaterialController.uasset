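; Material controller component that gives a static mesh a randomized look through a dynamic material instance.
; UpdateMaterial stores the passed mesh and particle system, then randomizes base color, pattern mask texture and mask color, using configurable ranges for both colors.
; A random roll enables tessellation with a random world displacement about half the time.
; Particle and trail color randomization exists but is disconnected, so the particle system stays untouched.
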(event Custom|UpdateMaterial
  (params (StaticMesh :type Static%20Mesh%20Object%20Reference) (ParticleSystem :type Particle%20System%20Object%20Reference))
  (bind _patronesarray (Variables|Default|GetPatronesArray))
  (bind _minrangecolor (Variables|Default|GetMinRangeColor))
  (bind _maxrangecolor (Variables|Default|GetMaxRangeColor))
  (bind _minrangecolormask (Variables|Default|GetMinRangeColorMask))
  (bind _maxrangecolormask (Variables|Default|GetMaxRangeColorMask))
  (Variables|Default|SetStaticMesh StaticMesh)
  (Variables|Default|SetParticleSystem ParticleSystem)
  (Utilities|FlowControl|Sequence
    (:then_0
      ;[1 1 1] Random Color Por Rangos
      (bind _returnvalue (Rendering|Material|CreateDynamicMaterialInstance (Rendering|Material|GetMaterial (Variables|Default|GetStaticMesh) 0) :!class /Script/Engine.KismetMaterialLibrary))
      (Variables|Default|SetMElementoBaseInst _returnvalue)
      (Rendering|Material|SetVectorParameterValue _returnvalue "Color" (Math|Conversions|ToLinearColor(Vector) (Math|Vector|MakeVector (Math|Random|RandomFloatinRange _minrangecolor _maxrangecolor) (Math|Random|RandomFloatinRange _minrangecolor _maxrangecolor) (Math|Random|RandomFloatinRange _minrangecolor _maxrangecolor))) :!class /Script/Engine.MaterialInstanceDynamic)
      (Rendering|Material|SetMaterial 0 0)
      ;[1 1 1] Coge una mascara de patrones random del array y lo aplica al material
      (Rendering|Material|SetTextureParameterValue _returnvalue "PatronesMascara" (Utilities|Array|Get(acopy) _patronesarray (Math|Random|RandomIntegerinRange 0 (Utilities|Array|Length _patronesarray))))
      ;[1 1 1] Color Random a la mascara por rangos
      (Rendering|Material|SetVectorParameterValue _returnvalue "ColorMascara" (Math|Conversions|ToLinearColor(Vector) (Math|Vector|MakeVector (Math|Random|RandomFloatinRange _minrangecolormask _maxrangecolormask) (Math|Random|RandomFloatinRange _minrangecolormask _maxrangecolormask) (Math|Random|RandomFloatinRange _minrangecolormask _maxrangecolormask))) :!class /Script/Engine.MaterialInstanceDynamic)
      (Math|Float|CompareFloat (Math|Random|RandomFloatinRange -1.0 1.0) 0.0
        (:>
          (Rendering|Material|SetScalarParameterValue _returnvalue "Tesselation?" 1.0 :!class /Script/Engine.MaterialInstanceDynamic)
          (Rendering|Material|SetScalarParameterValue _returnvalue "WorldDispacement" (Math|Random|RandomFloatinRange 1.0 5.0) :!class /Script/Engine.MaterialInstanceDynamic))))))

(event EventBeginPlay)