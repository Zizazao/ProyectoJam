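; BP_Seed is a seed actor that can be grabbed, using a fixed round grab animation on its static mesh.
; On BeginPlay it spawns a BP_SeedComponentCollision at each mesh socket and snaps it to that socket.
; The end of an overlap on SM_Seed releases the Grabable component.
; Construction-script socket attachment and a mesh fusion call remain as unconnected nodes.
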(event OnComponentBeginOverlap(SM_Seed)
  (params (OverlappedComponent :type Primitive%20Component%20Object%20Reference) (OtherActor :type Actor%20Object%20Reference) (OtherComp :type Primitive%20Component%20Object%20Reference) (OtherBodyIndex :type Integer) (bFromSweep :type Boolean) (SweepResult :type Hit%20Result%20Structure%20%28by%20ref%29)))

(event OnComponentEndOverlap(SM_Seed)
  (params (OverlappedComponent :type Primitive%20Component%20Object%20Reference) (OtherActor :type Actor%20Object%20Reference) (OtherComp :type Primitive%20Component%20Object%20Reference) (OtherBodyIndex :type Integer))
  (Default|Released (Variables|Default|GetGrabable)))

(event EventBeginPlay
  (bind _sm_seed (Variables|Default|GetSM_Seed))
  ;[1 1 1] Para Agarrar la semilla
  (Default|SetFixedGrab :self (Variables|Default|GetGrabable) :Volume (Variables|Default|GetSM_Seed) :Animation "/Game/Framework/Hands/Model/Animations/Grabs/grab_round_medium.grab_round_medium")
  (for _array_element (Transformation|GetAllSocketNames _sm_seed)
    ;[1 0.1872 0.1823] Ajustar Class BP
    (bind _returnvalue (Game|SpawnActorfromClass "/Game/Blueprints/Seed/Components/BP_SeedComponentCollision.BP_SeedComponentCollision_C" (Transformation|GetSocketTransform _sm_seed _array_element "RTS_Component") "Undefined" 0 0))
    (Variables|Default|SetRef:Mesh (Actor|GetComponentbyClass _returnvalue "/Script/Engine.StaticMeshComponent"))
    (Transformation|AttachComponentToComponent _returnvalue (Variables|Default|GetSM_Seed) _array_element "SnapToTarget" "SnapToTarget" "SnapToTarget" true)))

(fn ConstructionScript)