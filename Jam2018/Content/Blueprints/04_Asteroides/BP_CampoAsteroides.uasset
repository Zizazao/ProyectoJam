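; Asteroid field actor that spawns a set number of BP_Asteroide actors at BeginPlay and slowly or variably rotates by timeline.
; Spawn positions use random circle-equation math around the root with RadioCampo, plus random outward offsets up to RadioExterior and slight height variation.
; Each scaled-up asteroid's root is attached with snap-to-target rules.
; Tick plays the GiroCampo timeline, whose track drives the actor's yaw rotation.
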(event EventBeginPlay
  (bind _radiocampo (Variables|Default|GetRadioCampo))
  (bind _radiocampo_2 (Variables|Default|GetRadioCampo))
  (bind _radiocampo_3 (Variables|Default|GetRadioCampo))
  (bind _defaultsceneroot (Variables|Default|GetDefaultSceneRoot))
  (bind _returnvalue (Transformation|GetWorldLocation _defaultsceneroot))
  (bind _returnvalue_2 (* _radiocampo_3 _radiocampo_2))
  (bind _returnvalue_3 (* _radiocampo -1.0))
  (bind _returnvalue_4 (Math|Random|RandomFloatinRange _returnvalue_3 _radiocampo))
  (bind _returnvalue_5 (* _returnvalue_4 _returnvalue_4))
  (bind _returnvalue_6 (- _returnvalue_2 _returnvalue_5))
  (bind _returnvalue_7 (Math|Float|Sqrt _returnvalue_6))
  (Utilities|FlowControl|Sequence
    (:then_0
      (for _index (range 0 (Variables|Default|GetAsteroidesTotal))
        (bind _returnvalue_8 (Game|SpawnActorfromClass "/Game/Blueprints/04_Asteroides/BP_Asteroide.BP_Asteroide_C" (Math|Transform|MakeTransform (Math|Vector|MakeVector (+ (Math|Random|RandomFloatinRange 0.0 (Variables|Default|GetRadioExterior)) (+ (.x _returnvalue) _returnvalue_4)) (+ (Math|Float|SelectFloat (+ (.y _returnvalue) _returnvalue_7) (- (.y _returnvalue) _returnvalue_7) (Math|Random|RandomBool)) (Math|Random|RandomFloatinRange 0.0 (Variables|Default|GetRadioExterior))) (Math|Random|RandomFloatinRange -1e+02 1e+02)) "0, 0, 0" "10.000000,10.000000,10.000000") "Undefined" 0 0))
        (Transformation|AttachComponentToComponent (Variables|/Game/Blueprints/04_Asteroides/BP_Asteroide.BP_Asteroide_C|GetDefaultSceneRoot _returnvalue_8) 0 "None" "SnapToTarget" "SnapToTarget" "SnapToTarget" true)))))

(event EventTick
  (params (DeltaSeconds :type Float%20%28single-precision%29))
  (bind _newtrack_0 (Timeline|giroCampo Play)
    (:Update
      (Class|Actor|AddActorWorldRotation (Math|Rotator|MakeRotator 0.0 0.0 _newtrack_0)))))

(fn ConstructionScript)